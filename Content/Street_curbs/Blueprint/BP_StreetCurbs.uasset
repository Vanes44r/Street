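; BP_StreetCurbs is a construction-script tool that lays out a straight row of street curb pieces.
; It gathers its InstancedStaticMesh components and picks one at random for each instance, mixing mesh variants along the row.
; The first piece sits at the origin, and CountCurbs drives further pieces at fixed spacing along local X with slight random roll and pitch.
; The event graph has no gameplay logic.
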(event EventBeginPlay)

(event Collision|EventActorBeginOverlap
  (params (OtherActor :type Actor%20Object%20Reference)))

(event EventTick
  (params (DeltaSeconds :type Float%20%28single-precision%29)))

(fn ConstructionScript
  (bind _output_get (Variables|Default|SetISMs (Actor|GetComponentsByClass "/Script/Engine.InstancedStaticMeshComponent")))
  (Components|InstancedStaticMesh|AddInstance (.OutItem (Utilities|Array|Random _output_get)) (Math|Transform|MakeTransform "0, 0, 0" "0, 0, 0" "1.000000,1.000000,1.000000") false)
  (for _index (range 0 (Variables|Default|GetCountCurbs))
    (if (!= _index 0)
      (Components|InstancedStaticMesh|AddInstance (.OutItem (Utilities|Array|Random (Variables|Default|GetISMs))) (Math|Transform|MakeTransform (Math|Vector|MakeVector (Math|Conversions|ToFloat(Integer) (+ 0 (* _index 103))) 0.0 0.0) (Math|Rotator|MakeRotator (Math|Random|RandomFloatinRange -5.0 5.0) (Math|Random|RandomFloatinRange -0.5 0.5) 0.0) "1.000000,1.000000,1.000000") false))))